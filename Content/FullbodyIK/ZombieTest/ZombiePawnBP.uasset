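; Zombie test pawn for full-body IK that targets the VR player and sets up physical animation on its skeletal mesh.
; Shortly after BeginPlay it stores the player's BP_VRCharacter as TargetVictim, then initializes physics only if that cast succeeds.
; Initialization runs DragonIKPhysics first-time setup, simulates bodies from spine_01 down the bone chain, then caches the simulation states.
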(event `Physanim Initialize`
  (bind _dragonikphysics (`self.DragonIKPhysics`))
  (bind _skeletalmesh (`self.SkeletalMesh`))
  (`DragonIKPhysicsComponent.FirstTimeInitialization` _dragonikphysics _skeletalmesh)
  (`SkeletalMeshComponent.SetAllBodiesBelowSimulatePhysics` _skeletalmesh "spine_01" true true)
  (`DragonIKPhysicsComponent.CacheSimulationStates` _dragonikphysics))

(event `self.ReceiveBeginPlay`
  (`KismetSystemLibrary.Delay` 0.2)
  (bind _asbp_vrcharacter (cast `/Game/VRE/Core/Character/BP_VRCharacter` (`GameplayStatics.GetPlayerPawn` 0)))
  (set `self.TargetVictim` _asbp_vrcharacter)
  (`self.Physanim Initialize`))

(fn `UserConstructionScript`)